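; BP_Enemy is a simple enemy that chases the player once within aggro range.
; Each tick it picks Idle, Walking or melee Attacking from its distance to player pawn 0, compared against AggroRange and MeleeRange.
; Walking yaws the capsule toward the player and moves forward at half input, without navigation or pathfinding.
; Melee Attacking only turns to face the player, with no attack logic in this Blueprint.
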(event `self.ReceiveTick`
  (params (DeltaSeconds :type "Float (single-precision)"))
  (`self.SetEnemyState`)
  (switch `/Game/HonestJam/Blueprints/EnemyState` (`self.EnemyState`)
    (:`NewEnumerator1`
      (`self.LookAtPlayer`)
      (`self.AddMovementInput` (`SceneComponent.GetForwardVector` (`self.CapsuleComponent`)) 0.5))
    (:`NewEnumerator2`
      (`self.LookAtPlayer`))))

(fn `GetDistanceToPlayer`
  (returns (DistanceToPlayer :type "Float (double-precision)"))
  (return (`self.GetDistanceTo` (`GameplayStatics.GetPlayerPawn` 0))))

(fn `LookAtPlayer`
  (bind (_returnvalue_roll _returnvalue_pitch _returnvalue_yaw) (`KismetMathLibrary.BreakRotator` (`KismetMathLibrary.FindLookAtRotation` (`self.K2_GetActorLocation` self) (`self.K2_GetActorLocation` (`GameplayStatics.GetPlayerPawn` 0)))))
  (`SceneComponent.K2_SetWorldRotation` (`self.CapsuleComponent`) (`KismetMathLibrary.MakeRotator` 0.0 0.0 _returnvalue_yaw) false false))

(fn `SetEnemyState`
  (if (<= (`self.GetDistanceToPlayer`) (`self.AggroRange`))
    (if (<= (`self.GetDistanceToPlayer`) (`self.MeleeRange`))
      (set `self.EnemyState` "NewEnumerator2")
      (else
        (set `self.EnemyState` "NewEnumerator1")))
    (else
      (set `self.EnemyState` "NewEnumerator0"))))

(fn `UserConstructionScript`)