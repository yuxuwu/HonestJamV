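; BP_MeleeWeaponV2 is a melee weapon pickup that attaches to the character and registers itself on BP_FirstPersonCharacter.
; An attack from the melee component starts a fast looping timer that line traces between the Tip and Handle sockets, with debug drawing.
; Every trace applies fixed damage to the hit actor, with no filter against repeat hits.
; NotifyAnimFinish clears the timer to end the damage window.
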(event `self.TP_PickUp.OnPickUp`
  (params (PickUpCharacter :type "HonestJamVCharacter Object Reference"))
  (`Comp_MeleeWeapon.AttachWeapon` (`self.Comp_MeleeWeapon`) PickUpCharacter)
  (bind _asbp_first_person_character (cast `/Game/FirstPerson/Blueprints/BP_FirstPersonCharacter` PickUpCharacter))
  (set `/Game/FirstPerson/Blueprints/BP_FirstPersonCharacter.WeaponPickedUp` self _asbp_first_person_character))

(event `self.Comp_MeleeWeapon.OnAttack`
  (`KismetSystemLibrary.PrintString` "Hello")
  (bind _returnvalue (`KismetSystemLibrary.K2_SetTimerDelegate` (delegate `MeleeWeaponLineTrace`) 0.01 true))
  (set `self.TriggerSwordEvent` _returnvalue))

(event `/Game/HonestJams/BPI_AnimNotify.NotifyAnimFinish`
  (`KismetSystemLibrary.K2_ClearAndInvalidateTimerHandle` (`self.TriggerSwordEvent`)))

(event `MeleeWeaponLineTrace`
  (bind _comp_meleeweapon (`self.Comp_MeleeWeapon`))
  (bind _outhit (`KismetSystemLibrary.LineTraceSingle` :`Start` (`SceneComponent.GetSocketLocation` _comp_meleeweapon "Tip") :`End` (`SceneComponent.GetSocketLocation` _comp_meleeweapon "Handle") :`TraceChannel` "TraceTypeQuery2" :`DrawDebugType` "ForDuration"))
  (`GameplayStatics.ApplyDamage` (`.HitActor` (`GameplayStatics.BreakHitResult` _outhit)) 10.0))

(fn `UserConstructionScript`)