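; Crossbow bolt projectile that damages BP_Dummy targets when its Box overlaps them, ignoring all other actors.
; On a hit it applies fixed damage, then waits a brief delay before calling AttachArrow and StopArrowPlaySounds.
; AttachArrow attaches the dummy to the Bolt component, keeping world transforms.
; StopArrowPlaySounds halts projectile movement, plays the impact sound, disables Bolt collision and destroys the Box.
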(event `self.Box.OnComponentBeginOverlap`
  (params (OverlappedComponent :type "PrimitiveComponent Object Reference") (OtherActor :type "Actor Object Reference") (OtherComp :type "PrimitiveComponent Object Reference") (OtherBodyIndex :type Integer) (bFromSweep :type Boolean) (SweepResult :type "HitResult Structure (by ref)"))
  (bind _asbp_dummy (cast `/Game/HonestJams/Enemies/BP_Dummy` OtherActor))
  (`GameplayStatics.ApplyDamage` _asbp_dummy 10.0 null self)
  (`|ExecutionSequence`
    (:`then_0`
      (`KismetSystemLibrary.Delay` 0.035)
      (`self.AttachArrow` _asbp_dummy)
      (`self.StopArrowPlaySounds`))))

(fn `AttachArrow`
  (params (InputPin :type "/Game/HonestJams/Enemies/BP_Dummy Object Reference"))
  (bind _bolt (`self.Bolt`))
  (`/Engine/EditorBlueprintResources/StandardMacros.IsValid` _bolt
    (:`Is Valid`
      (`/Engine/EditorBlueprintResources/StandardMacros.IsValid` InputPin
        (:`Is Valid`
          (`self.K2_AttachToComponent` InputPin _bolt "None" "KeepWorld" "KeepWorld" "KeepWorld" true))))))

(fn `StopArrowPlaySounds`
  (`MovementComponent.StopMovementImmediately` (`self.ProjectileMovement`))
  (`GameplayStatics.PlaySoundAtLocation` "/Game/Assets/Crossbow/Sounds/Bolt_Impact_Cue.Bolt_Impact_Cue" (`self.K2_GetActorLocation`) (struct) 1.0 1.0 0.0 null null null null)
  (`PrimitiveComponent.SetCollisionEnabled` (`self.Bolt`) "NoCollision")
  (`ActorComponent.K2_DestroyComponent` (`self.Box`)))

(fn `UserConstructionScript`)