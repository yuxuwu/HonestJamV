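; Melee weapon that BP_BrandonFirstPerson picks up, attaches if no crossbow is held, and can drop as a physics object.
; Attacks run a looping timer that traces between blade Tip and Handle sockets, with a DoOnce limiting damage to once per swing until the finish notify resets it.
; Hits on BP_Dummy play hit or kill sounds.
; Blocking uses a similar timer to set a blocking flag until its finish notify.
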(event `self.TP_PickUp.OnPickUp`
  (params (PickUpCharacter :type "HonestJamVCharacter Object Reference"))
  (`self.AttachWeapon` PickUpCharacter (`HonestJamVCharacter.bHasCrossbow` PickUpCharacter))
  (`self.SetCharacter` PickUpCharacter))

(event `/Game/HonestJams/Interfaces/BPI_WeaponsInteract.DropWeapon`
  (`SceneComponent.K2_DetachFromComponent` (`self.Comp_MeleeWeapon`) "KeepWorld" "KeepWorld" "KeepWorld" true)
  (`self.OnDropped`))

(event `self.Comp_MeleeWeapon.OnAttack`
  (`GameplayStatics.PlaySoundAtLocation` "/Game/Assets/Sword/Sword_Attack.Sword_Attack" (`self.K2_GetActorLocation`) (struct) 1.0 1.0 0.0 null null null null)
  (bind _returnvalue (`KismetSystemLibrary.K2_SetTimerDelegate` (delegate `MeleeWeaponLineTrace`) 0.01 true))
  (set `self.AttackTimeHandle` _returnvalue))

(event `/Game/HonestJams/Interfaces/BPI_WeaponsInteract.NotifyAttackFinished`
  (`KismetSystemLibrary.K2_ClearAndInvalidateTimerHandle` (`self.AttackTimeHandle`))
  (goto _label :!via `Reset`))

(event `MeleeWeaponLineTrace`
  (bind _outhit (`self.TraceHit`))
  (bind (_bblockinghit _binitialoverlap _time _distance _location _impactpoint _normal _impactnormal _physmat _hitactor) (`GameplayStatics.BreakHitResult` _outhit))
  (if _bblockinghit
    (`/Engine/EditorBlueprintResources/StandardMacros.DoOnce` false :!label _label
      (:`Completed`
        (`GameplayStatics.ApplyDamage` _hitactor 10.0 null self)
        (`self.PlaySoundHitDummy` _hitactor)))))

(event `self.Comp_MeleeWeapon.OnBlock`
  (bind _returnvalue (`KismetSystemLibrary.K2_SetTimerDelegate` (delegate `Block Collioin Enable`) 0.01 true))
  (set `self.BlockTimeHandle` _returnvalue))

(event `Block Collioin Enable`
  (set `self.IsBlocking` true))

(event `/Game/HonestJams/Interfaces/BPI_WeaponsInteract.NotifyBlockFinished`
  (`KismetSystemLibrary.K2_ClearAndInvalidateTimerHandle` (`self.BlockTimeHandle`))
  (set `/Game/HonestJams/Character/BP_BrandonFirstPerson.IsBlocking` false (`self.FP_Character`)))

(fn `AttachWeapon`
  (params (InputPin :type "HonestJamVCharacter Object Reference") (Condition :type Boolean))
  (if (not Condition)
    (`Comp_MeleeWeapon.AttachWeapon` (`self.Comp_MeleeWeapon`) InputPin)))

(fn `OnDropped`
  (bind _fp_character (`self.FP_Character`))
  (bind _comp_meleeweapon (`self.Comp_MeleeWeapon`))
  (`|ExecutionSequence`
    (:`then_0`
      (`PrimitiveComponent.SetSimulatePhysics` _comp_meleeweapon true))
    (:`then_1`
      (`PrimitiveComponent.SetEnableGravity` _comp_meleeweapon true))
    (:`then_2`
      (`PrimitiveComponent.SetCollisionEnabled` _comp_meleeweapon "PhysicsOnly"))
    (:`then_3`
      (`PrimitiveComponent.SetCollisionResponseToAllChannels` _comp_meleeweapon "ECR_Block"))
    (:`then_4`
      (`PrimitiveComponent.SetCollisionResponseToChannel` _comp_meleeweapon "ECC_Pawn" "ECR_Ignore"))
    (:`then_5`
      (`HonestJamVCharacter.SetHasMeleeWeapon` _fp_character false)
      (set `/Game/HonestJams/Character/BP_BrandonFirstPerson.CrossbowPickedUp` null _fp_character))))

(fn `PlaySoundHitDummy`
  (params (Object :type "Object Object Reference"))
  (bind _returnvalue (`self.K2_GetActorLocation`))
  (bind _asbp_dummy (cast `/Game/HonestJams/Enemies/BP_Dummy` Object))
  (if (<= (`/Game/HonestJams/Enemies/BP_Dummy.Health` _asbp_dummy) 0.0)
    (`GameplayStatics.PlaySoundAtLocation` "/Game/Assets/Sword/Sword_Kill_Cue.Sword_Kill_Cue" _returnvalue (struct) 1.0 1.0 0.0 null null null null)
    (else
      (`GameplayStatics.PlaySoundAtLocation` "/Game/Assets/Sword/Sword_hit_Cue.Sword_hit_Cue" _returnvalue (struct) 1.0 1.0 0.0 null null null null))))

(fn `SetCharacter`
  (params (Object :type "Object Object Reference"))
  (bind _asbp_brandon_first_person (cast `/Game/HonestJams/Character/BP_BrandonFirstPerson` Object))
  (bind _output_get (set `self.FP_Character` _asbp_brandon_first_person))
  (set `/Game/HonestJams/Character/BP_BrandonFirstPerson.WeaponPickedUp` self _output_get)
  (`self.SetOwner` _output_get))

(fn `TraceHit`
  (returns (OutHit :type "HitResult Structure"))
  (bind _comp_meleeweapon (`self.Comp_MeleeWeapon`))
  (bind _outhit (`KismetSystemLibrary.LineTraceSingle` (`SceneComponent.GetSocketLocation` _comp_meleeweapon "Tip") (`SceneComponent.GetSocketLocation` _comp_meleeweapon "Handle") "TraceTypeQuery2" false (`|MakeArray` (`self.FP_Character`) :!type "Actor Object Reference") "ForDuration"))
  (return _outhit))

(fn `UserConstructionScript`)