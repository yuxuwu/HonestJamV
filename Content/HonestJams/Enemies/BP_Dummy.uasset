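; BP_Dummy is a target dummy enemy that tracks its health and prints it to show the effect of hits.
; Health starts at MaxHealth on BeginPlay.
; AnyDamage accepts damage only when the causer casts to BP_MeleeWeapon or BP_CrossbowBolt, with both branches sharing one clamped subtraction and print.
; It has no death handling, so Health simply bottoms out at zero.
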(event `self.ReceiveBeginPlay`
  (set `self.Health` (`self.MaxHealth`))
  (`KismetSystemLibrary.PrintString` (`KismetStringLibrary.Conv_DoubleToString` (`self.Health`))))

(event `self.ReceiveAnyDamage`
  (params (Damage :type "Float (single-precision)") (DamageType :type "DamageType Object Reference") (InstigatedBy :type "Controller Object Reference") (DamageCauser :type "Actor Object Reference"))
  (`|ExecutionSequence`
    (:`then_0`
      (cast `/Game/HonestJams/Weapon/BP_MeleeWeapon` DamageCauser))
    (:`then_1`
      (cast `/Game/HonestJams/Weapon/BP_CrossbowBolt` DamageCauser)))
  (bind _output_get (set `self.Health` (`KismetMathLibrary.FClamp` (- (`self.Health`) Damage) 0.0 (`self.MaxHealth`))))
  (`KismetSystemLibrary.PrintString` (`KismetStringLibrary.Conv_DoubleToString` _output_get)))

(fn `UserConstructionScript`)